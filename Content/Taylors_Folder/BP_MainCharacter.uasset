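; BP_MainCharacter is a character Blueprint that lets the player shrink or grow a GreenHerb actor when close to it.
; Each Tick finds a GreenHerb via GetActorOfClass and sets CanInteract when it lies within a fixed distance of the character.
; While CanInteract is true, the 1 and 2 keys look up the herb again and call its Shrink and Grow respectively.
; The lookup returns a single actor, so only one herb is considered, not necessarily the nearest.
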(event EventTick
  (params (DeltaSeconds :type Float%20%28single-precision%29))
  (bind _returnvalue (Actor|GetActorOfClass "/Game/Taylors_Folder/HerbBlueprints/GreenHerb.GreenHerb_C"))
  (Variables|Default|SetCanInteract (<= (Math|Vector|Distance(Vector) (Transformation|GetActorLocation) (Transformation|GetActorLocation _returnvalue)) 5e+02)))

(event Input|KeyboardEvents|1
  (params (Key :type Key%20Structure :default "None"))
  (:Pressed
    (if (Variables|Default|GetCanInteract)
      (bind _returnvalue (Actor|GetActorOfClass "/Game/Taylors_Folder/HerbBlueprints/GreenHerb.GreenHerb_C"))
      (Class|FloraInterface|Shrink _returnvalue))))

(event Input|KeyboardEvents|2
  (params (Key :type Key%20Structure :default "None"))
  (:Pressed
    (if (Variables|Default|GetCanInteract)
      (bind _returnvalue (Actor|GetActorOfClass "/Game/Taylors_Folder/HerbBlueprints/GreenHerb.GreenHerb_C"))
      (Class|FloraInterface|Grow _returnvalue))))

(fn ConstructionScript)